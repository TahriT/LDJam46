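; Dodo cannon turret that turns toward a seen Twin pawn's LeftActor and fires scaled-up Dodo projectiles from TurretMouth.
; A Delay gate limits shots to FireRate and drives the anim blueprint's ShouldFire on Tick; each shot also impulses the turret's own mesh.
; TwinStickProjectile hits apply point damage, set the health bar before reducing Hp, then reach a destroy check that compares Hp to itself, so never passes.
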(event OnSeePawn(PawnSensing)
  (params (Pawn :type Pawn%20Object%20Reference))
  (bind _astwin (Utilities|Casting|CastToTwin Pawn))
  (Utilities|FlowControl|Sequence
    (:then_0
      (Transformation|SetActorRotation (Math|Rotator|FindLookatRotation (Transformation|GetActorLocation self) (Transformation|GetActorLocation (Variables|/Game/TwinStickBP/Blueprints/Twin.Twin_C|GetleftActor _astwin)))))
    (:then_1
      (if (Variables|Default|GetcanSpawnProjectile)
        (bind _returnvalue (Game|SpawnActorfromClass "/Game/TwinStickBP/Blueprints/dodo_projectile.dodo_projectile_C" (Transformation|GetWorldTransform (Variables|Default|GetturretMouth)) "AlwaysSpawn" 0 0))
        (Transformation|SetActorScale3D _returnvalue (* "1.000000,1.000000,1.000000" 5.0))
        (Physics|AddImpulse (Variables|Default|GetSkeletalMesh) (* (Math|Vector|GetForwardVector (Variables|Default|GetSkeletalMesh)) (Variables|Default|GetbulletImpulse)) "None" true)
        (Variables|Default|SetcanSpawnProjectile false)
        (Utilities|FlowControl|Delay (/ 1.0 (Variables|Default|GetfireRate)))
        (Variables|Default|SetcanSpawnProjectile true)))))

(event OnComponentHit(SkeletalMesh)
  (params (HitComponent :type Primitive%20Component%20Object%20Reference) (OtherActor :type Actor%20Object%20Reference) (OtherComp :type Primitive%20Component%20Object%20Reference) (NormalImpulse :type Vector :default "0, 0, 0") (Hit :type Hit%20Result%20Structure%20%28by%20ref%29))
  (bind (_bblockinghit _binitialoverlap _time _distance _location _impactpoint _normal _impactnormal _physmat _hitactor) (Collision|BreakHitResult Hit))
  (Utilities|Casting|CastToTwinStickProjectile OtherActor)
  (bind _returnvalue (Game|Damage|ApplyPointDamage _hitactor 1e+02 _impactpoint Hit))
  (bind _ashealth_bar (Utilities|Casting|CastToHealthBar (UserInterface|GetUserWidgetObject (Variables|Default|GetWidget))))
  (Progress|SetPercent (Variables|/Game/Sandbox/Crab_Castle_Crisis/UI/HealthBar.HealthBar_C|GetProgressBar_91 _ashealth_bar) (/ (Variables|Default|Gethp) (Variables|Default|GetMaxhp)))
  (bind _output_get (Variables|Default|Sethp (Math|Conversions|ToFloat(Integer) (- (Math|Float|Truncate (Variables|Default|Gethp)) (Math|Float|Truncate _returnvalue)))))
  (if (< (Math|Float|Truncate _output_get) (Math|Float|Truncate (Variables|Default|Gethp)))
    (Actor|DestroyActor self)))

(event EventBeginPlay)

(event Collision|EventActorBeginOverlap
  (params (OtherActor :type Actor%20Object%20Reference)))

(event EventTick
  (params (DeltaSeconds :type Float%20%28single-precision%29))
  (bind _asdodo_turret_anim_bp (Utilities|Casting|CastToDodoTurretAnimBP (Components|SkeletalMesh|GetAnimInstance (Variables|Default|GetSkeletalMesh))))
  (Variables|/Game/Geometry/GameModels/DodoRedo/DodoTurretAnimBP.DodoTurretAnimBP_C|SetShouldFire _asdodo_turret_anim_bp (Variables|Default|GetcanSpawnProjectile)))

(fn ConstructionScript)