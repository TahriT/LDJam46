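; BP_Dodo_Spawner is a spawner actor that keeps adding AI BP_DodoCannon pawns while their world count is below MaxSpawn.
; Tick checks that count and, after a one-second Delay, runs SpawnCrab SpawnCount times.
; SpawnCrab picks a random point inside the Bound component's bounds, with rotation looking from Bound toward TwinRef.
; It passes AttackLeftPlayer to the spawned pawn only if the cast to BP_Crab succeeds.
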(event Collision|EventActorBeginOverlap
  (params (OtherActor :type Actor%20Object%20Reference)))

(event EventTick
  (params (DeltaSeconds :type Float%20%28single-precision%29))
  (Utilities|FlowControl|Sequence
    (:then_0
      (bind _outactors (Actor|GetAllActorsOfClass "/Game/Sandbox/Shah/BP_DodoCannon.BP_DodoCannon_C"))
      (if (< (Utilities|Array|Length _outactors) (Variables|Default|GetMax%20Spawn))
        (Utilities|FlowControl|Delay 1.0)
        (for _index (range 1 (Variables|Default|GetspawnCount))
          (CallFunction|SpawnCrab))))))

(fn ConstructionScript)

(fn SpawnCrab
  (bind _bound (Variables|Default|GetBound))
  (bind (_origin _boxextent) (Collision|GetComponentBounds _bound))
  (bind _returnvalue (AI|SpawnAIFromClass "/Game/Sandbox/Shah/BP_DodoCannon.BP_DodoCannon_C" 0 (Math|Random|RandomPointinBoundingBox _origin _boxextent) (Math|Rotator|FindLookatRotation (Transformation|GetWorldLocation _bound) (Transformation|GetActorLocation (Variables|Default|GetTwinRef))) false))
  (bind _asbp_crab (Utilities|Casting|CastToBP_Crab _returnvalue))
  (Variables|/Game/Sandbox/Shah/BP_Crab.BP_Crab_C|SetattackLeftPlayer _asbp_crab (Variables|Default|GetAttackLeftPlayer)))